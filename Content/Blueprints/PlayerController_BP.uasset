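; Player controller for a two-player score game that spawns the start, options or in-game widget based on the current level name.
; Point events blink the scoring player's counter text using delays and a repeat countdown.
; End-game events save the winner name to slot "1" and show the end widget.
; Options events adjust the win-condition points within bounds and save them to slot "2".
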(event `repeat`
  ;[1 1 1] Parpadeo de la Puntiación al marcar punto
  (set `self.counter1` "" :!label _label)
  (`KismetSystemLibrary.Delay` 0.2)
  (set `self.counter1` (`self.Supp`))
  (`KismetSystemLibrary.Delay` 0.2)
  (bind _result (`/Engine/EditorBlueprintResources/StandardMacros.DecrementInt` (`self.Repeticiones`))
    (:`  `
      (if (<= _result 0)
        (set `self.Repeticiones` 3)
        (else
          (`self.repeat`))))))

(event `PointDone`
  ;[1 1 1] Parpadeo de la Puntiación al marcar punto
  (set `self.Supp` (`self.counter1`))
  (goto _label))

(event `PointDone2`
  ;[1 1 1] Parpadeo de la Puntiación al marcar punto
  (set `self.Supp` (`self.counter2`))
  (set `self.counter2` "" :!label _label_2)
  (`KismetSystemLibrary.Delay` 0.2)
  (set `self.counter2` (`self.Supp`))
  (`KismetSystemLibrary.Delay` 0.2)
  (bind _result (`/Engine/EditorBlueprintResources/StandardMacros.DecrementInt` (`self.Repeticiones`))
    (:`  `
      (if (<= _result 0)
        (set `self.Repeticiones` 3)
        (else
          (`self.repeat2`))))))

(event `EndGame`
  (set `self.winName` "Player 1")
  ;[1 1 1] Guarda la información de la partida
  (bind _returnvalue (`GameplayStatics.CreateSaveGameObject` "/Game/Blueprints/SaveGame_BP.SaveGame_BP_C" :!label _label_3))
  (bind _output_get (set `self.SaveGame` _returnvalue))
  (set `/Game/Blueprints/SaveGame_BP.Winner` (`self.winName`) _output_get)
  (`GameplayStatics.SaveGameToSlot` (`self.SaveGame`) "1")
  (bind _returnvalue_2 (`|CreateWidget` "/Game/Blueprints/WIdgets/EndWidget_BP.EndWidget_BP_C"))
  (`UserWidget.AddToViewport` _returnvalue_2 0)
  (set `self.gameEnded` true))

(event `repeat2`
  ;[1 1 1] Parpadeo de la Puntiación al marcar punto
  (goto _label_2))

(event `addWincondition`
  (params (points :type Integer))
  (bind _output_get (set `self.WinCondition` points))
  (if (> 99 _output_get)
    (`/Engine/EditorBlueprintResources/StandardMacros.IncrementInt` _output_get)))

(event `StartGame`
  (`GameplayStatics.OpenLevel` "Map_01")
  (set `self.bShowMouseCursor` false))

(event `lessWincondition`
  (params (points :type Integer))
  (bind _output_get (set `self.WinCondition` points))
  (if (> _output_get 1)
    (`/Engine/EditorBlueprintResources/StandardMacros.DecrementInt` _output_get)))

(event `saveOptions`
  (bind _returnvalue (`GameplayStatics.CreateSaveGameObject` "/Game/Blueprints/SaveGame_BP.SaveGame_BP_C"))
  (bind _output_get (set `self.SaveGame` _returnvalue))
  (set `/Game/Blueprints/SaveGame_BP.Points` (`self.WinCondition`) _output_get)
  (`GameplayStatics.SaveGameToSlot` _output_get "2"))

(event `EndGame2`
  (set `self.winName` "Player 2")
  (goto _label_3))

(event `self.ReceiveBeginPlay`
  ;[1 1 1] Crear Widget dependiendo del Mapa
  (bind _returnvalue (`GameplayStatics.GetCurrentLevelName` true))
  (if (`KismetStringLibrary.EqualEqual_StrStr` _returnvalue "Map_01")
    (bind _returnvalue_2 (`|CreateWidget` "/Game/Blueprints/WIdgets/PlayerWidget.PlayerWidget_C"))
    (`UserWidget.AddToViewport` _returnvalue_2 0)
    (elif (`KismetStringLibrary.EqualEqual_StrStr` _returnvalue "Start")
      (bind _returnvalue_3 (`|CreateWidget` "/Game/Blueprints/WIdgets/StartWidget.StartWidget_C" self))
      (`UserWidget.AddToViewport` _returnvalue_3 0)
      (set `self.bShowMouseCursor` true)
      (elif (`KismetStringLibrary.EqualEqual_StrStr` _returnvalue "Options")
        (bind _returnvalue_4 (`|CreateWidget` "/Game/Blueprints/WIdgets/OptionsWIdget.OptionsWIdget_C"))
        (`UserWidget.AddToViewport` _returnvalue_4 0)))))

(fn `UserConstructionScript`)