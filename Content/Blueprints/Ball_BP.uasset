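; Ball actor for a two-player Pong-style game that bounces, tracks both scores and ends the match.
; StartPlay launches it at a randomly yawed angle; hits reflect its stored direction with slight random jitter at constant Speed.
; Goal triggers, matched by object name, increment scores, reset and relaunch the ball after a delay, and update PlayerController_BP.
; Reaching the points target loaded from SaveGame_BP calls that controller's end-game event and destroys the ball.
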(event `PointOn`
  ;[1 1 1] vuelve a empezar tras marcar punto
  (`PrimitiveComponent.SetPhysicsLinearVelocity` (`self.Sphere`) (0.0 0.0 0.0) false "None")
  (`SceneComponent.K2_SetWorldLocation` (`self.Sphere`) (`self.K2_GetActorLocation` (`self.StartPoint`)) false false)
  (`KismetSystemLibrary.Delay` 1.6)
  ;[1 1 1] Presienar espacio para inicar el movimiento de la pelota
  (`PrimitiveComponent.SetPhysicsLinearVelocity` (`self.Sphere`) (* (`KismetMathLibrary.GreaterGreater_VectorRotator` (`SceneComponent.GetRightVector` (`self.Sphere`)) (`KismetMathLibrary.MakeRotator` 0.0 0.0 (`KismetMathLibrary.RandomFloatInRange` 5.0 30.0))) (`self.Speed`)) false "None" :!label _label)
  (set `/Game/Blueprints/PlayerController_BP.PressSpace` "" (`self.PlayerController`)))

(event `self.ReceiveBeginPlay`
  (bind _returnvalue (`GameplayStatics.DoesSaveGameExist` "2"))
  (if _returnvalue
    (bind _returnvalue_2 (`GameplayStatics.LoadGameFromSlot` "2"))
    (bind _assave_game_bp (cast `/Game/Blueprints/SaveGame_BP` _returnvalue_2)
      (:`then`
        (bind _output_get (set `self.SaveGame` _assave_game_bp))
        ;[1 1 1] Inicio del juego
        (set `self.wincondition` (`/Game/Blueprints/SaveGame_BP.Points` _output_get))
        (`self.EnableInput` (`GameplayStatics.GetPlayerController` 0))
        (bind _asplayer_controller_bp (cast `/Game/Blueprints/PlayerController_BP` (`GameplayStatics.GetPlayerController` 0)))
        (set `self.PlayerController` _asplayer_controller_bp)
        (set `self.Current Direction` (`KismetMathLibrary.GreaterGreater_VectorRotator` (`SceneComponent.GetRightVector` (`self.Sphere`)) (`KismetMathLibrary.MakeRotator` 0.0 0.0 (`KismetMathLibrary.RandomFloatInRange` 5.0 30.0)))))
      (:`CastFailed`
        (`KismetSystemLibrary.PrintString` "Fail")))))

(event `InputAction|StartPlay`
  (params (Key :type "Key Structure"))
  ;[1 1 1] Presienar espacio para inicar el movimiento de la pelota
  (:`Pressed`
    (if (`KismetStringLibrary.NotEqual_StrStr` (`/Game/Blueprints/PlayerController_BP.PressSpace` (`self.PlayerController`)))
      (goto _label))))

(event `self.ReceiveHit`
  (params (MyComp :type "PrimitiveComponent Object Reference") (Other :type "Actor Object Reference") (OtherComp :type "PrimitiveComponent Object Reference") (bSelfMoved :type Boolean) (HitLocation :type "Vector Structure") (HitNormal :type "Vector Structure") (NormalImpulse :type "Vector Structure") (Hit :type "HitResult Structure (by ref)"))
  ;[1 1 1] Cuando golpea un objeto
  (bind _output_get (set `self.Current Direction` (`KismetMathLibrary.GreaterGreater_VectorRotator` (`KismetMathLibrary.Normal` (`KismetMathLibrary.GetReflectionVector` (`self.Current Direction`) HitNormal)) (`KismetMathLibrary.MakeRotator` 0.0 0.0 (`KismetMathLibrary.RandomFloatInRange` -5.0 5.0)))))
  (`PrimitiveComponent.SetPhysicsLinearVelocity` (`self.Sphere`) (* _output_get (`self.Speed`)) false "None"))

(event `self.ReceiveActorBeginOverlap`
  (params (OtherActor :type "Actor Object Reference"))
  (bind _returnvalue (`KismetSystemLibrary.GetObjectName` OtherActor))
  (bind _point1 (`self.point1`))
  (bind _point2 (`self.point2`))
  (bind _playercontroller (`self.PlayerController`))
  (bind _playercontroller_2 (`self.PlayerController`))
  (bind _playercontroller_3 (`self.PlayerController`))
  ;[1 1 1] Entra en un trigger de puntiación
  (if (`KismetStringLibrary.EqualEqual_StrStr` _returnvalue "WinPlayer1")
    (bind _result (`/Engine/EditorBlueprintResources/StandardMacros.IncrementInt` _point1)
      (:`  `
        (if (== _result (`self.wincondition`))
          ;[1 1 1] Termina el juego
          (`/Game/Blueprints/PlayerController_BP.EndGame` (`self.PlayerController`))
          (set `/Game/Blueprints/PlayerController_BP.counter1` "" _playercontroller :!label _label_2)
          (set `/Game/Blueprints/PlayerController_BP.counter2` "" _playercontroller)
          (`self.K2_DestroyActor`)
          (else
            ;[1 1 1] Marca Punto
            (`self.PointOn`)
            (set `/Game/Blueprints/PlayerController_BP.counter1` (`KismetStringLibrary.Conv_IntToString` _point1) _playercontroller_2)
            (`/Game/Blueprints/PlayerController_BP.PointDone` _playercontroller_2)))))
    (elif (`KismetStringLibrary.EqualEqual_StrStr` _returnvalue "WinPlayer2_2")
      (bind _result_2 (`/Engine/EditorBlueprintResources/StandardMacros.IncrementInt` _point2)
        (:`  `
          (if (== _result_2 (`self.wincondition`))
            (`/Game/Blueprints/PlayerController_BP.EndGame2` (`self.PlayerController`))
            (goto _label_2)
            (else
              ;[1 1 1] Marca Punto
              (`self.PointOn`)
              (set `/Game/Blueprints/PlayerController_BP.counter2` (`KismetStringLibrary.Conv_IntToString` _point2) _playercontroller_3)
              (`/Game/Blueprints/PlayerController_BP.PointDone2` _playercontroller_3))))))))

(fn `UserConstructionScript`)