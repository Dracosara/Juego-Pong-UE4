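; Deplazador_2 is an actor moved by the Vertical_2 input axis, sliding along a straight line between the Top and Bottom marker actors.
; Axis input, scaled by Speed and delta time, accumulates into a clamped 0–1 Postion that linearly interpolates the location, without sweeping.
; Tick polls GameEnded on the first player's PlayerController_BP, disabling input when the game ends and enabling it otherwise.
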(event `self.ReceiveBeginPlay`
  (bind _asplayer_controller_bp (cast `/Game/Blueprints/PlayerController_BP` (`GameplayStatics.GetPlayerController` 0)))
  (set `self.playerController` _asplayer_controller_bp))

(event `self.ReceiveTick`
  (params (DeltaSeconds :type "Float (single-precision)"))
  (bind _playercontroller (`self.playerController`))
  ;[1 1 1] Se habilita la entrada
  (if (`/Game/Blueprints/PlayerController_BP.gameEnded` _playercontroller)
    (`self.DisableInput` _playercontroller)
    (else
      (`self.EnableInput` _playercontroller))))

(event `InputAxis|Vertical_2`
  (params (AxisValue :type "Float (single-precision)"))
  ;[1 1 1] Control de entrada
  ;[1 1 1] Interpolación de movimiento
  (bind _output_get (set `self.Postion` (`KismetMathLibrary.FClamp` (+ (* AxisValue (`self.Speed`) (`GameplayStatics.GetWorldDeltaSeconds`)) (`self.Postion`)))))
  (`self.K2_SetActorLocation` (`|EaseFunction` "Linear" _output_get (`self.K2_GetActorLocation` (`self.Top`)) (`self.K2_GetActorLocation` (`self.Bottom`)))))

(fn `UserConstructionScript`)